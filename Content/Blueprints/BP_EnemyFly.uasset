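; BP_EnemyFly is an enemy that damages the player character on contact and destroys itself in the process.
; A capsule hit on BP_Character applies its Damage value, while incoming damage reduces Health until the enemy is destroyed at zero or below.
; Both death paths first call UpdateEnemyLenght, which passes the enemy to BP_GameMode through EventUpdateEnemyLenght.
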(event `self.CapsuleComponent.OnComponentHit`
  (params (HitComponent :type "PrimitiveComponent Object Reference") (OtherActor :type "Actor Object Reference") (OtherComp :type "PrimitiveComponent Object Reference") (NormalImpulse :type "Vector Structure") (Hit :type "HitResult Structure (by ref)"))
  ;[1 1 1] Make Damage
  (bind _asbp_character (cast `/Game/Blueprints/BP_Character` OtherActor))
  (`GameplayStatics.ApplyDamage` _asbp_character (`self.Damage`) null self)
  (`self.Update Enemy Lenght` self)
  (`self.K2_DestroyActor`))

(event `self.ReceiveAnyDamage`
  (params (Damage :type "Float (single-precision)") (DamageType :type "DamageType Object Reference") (InstigatedBy :type "Controller Object Reference") (DamageCauser :type "Actor Object Reference"))
  ;[1 1 1] Enemy Hit
  (bind _output_get (set `self.Health` (- (`self.Health`) Damage)))
  (if (<= _output_get 0.0)
    (`self.Update Enemy Lenght` self)
    (`self.K2_DestroyActor`)))

(fn `Update Enemy Lenght`
  (params (Actor :type "Actor Object Reference"))
  (bind _asbp_game_mode (cast `/Game/Blueprints/BP_GameMode` (`GameplayStatics.GetGameMode`)))
  (`/Game/Blueprints/BP_GameMode.Event UpdateEnemyLenght` _asbp_game_mode Actor))

(fn `UserConstructionScript`)